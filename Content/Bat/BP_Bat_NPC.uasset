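; Bat NPC that flies around the level, lands on Fruit actors to eat, then resumes flight.
; Tick pushes the mesh forward and eases its rotation toward FlightTarget, which TurnBack repeatedly randomizes around an attractor before settling on it.
; Delayed box traces find nearby fruit, triggering moves onto its BatPlatform and a timed eating state.
; Otherwise, traces detect static obstacles and redirect the target to TurnBackPoint before wandering restarts.
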(event Custom|Turn%20Back
  (bind _attractor_location (Variables|Default|GetAttractor%20Location))
  (bind _max_flight_range (Variables|Default|GetMax%20Flight%20Range))
  (bind (_x _y _z) (Math|Vector|BreakVector _attractor_location))
  (bind _returnvalue (* _max_flight_range -1.0))
  (bind _returnvalue_2 (Math|Random|RandomFloatinRange _returnvalue _max_flight_range))
  (if (Variables|Default|GetFlying%20Forward?) :!label _label
    (Transformation|SetRelativeLocation (Variables|Default|GetFlight%20Target) (Math|Vector|MakeVector (+ _x _returnvalue_2) (+ _y _returnvalue_2) (+ _z (Math|Random|RandomFloatinRange (* _max_flight_range -0.2) _max_flight_range))) false false)
    (Variables|Default|SetTime%20in%20Flight (+ (Variables|Default|GetTime%20in%20Flight) 1))
    (Math|Integer|CompareInt (Variables|Default|GetTime%20in%20Flight) 12
      (:>
        _)
      (:==
        _)
      (:<
        (Utilities|FlowControl|Delay (Math|Random|RandomFloatinRange 2.0 4.0))
        (goto _label)))
    (Transformation|SetRelativeLocation (Variables|Default|GetFlight%20Target) (Variables|Default|GetAttractor%20Location) false false)))

(event EventTick
  (params (DeltaSeconds :type Float%20%28single-precision%29))
  (bind _mesh (Variables|Character|GetMesh))
  (bind _mesh_2 (Variables|Character|GetMesh))
  (bind _max_flight_range (Variables|Default|GetMax%20Flight%20Range))
  (bind _mesh_3 (Variables|Character|GetMesh))
  (bind _returnvalue (Transformation|GetWorldLocation _mesh))
  (bind _returnvalue_2 (Transformation|GetWorldLocation _mesh_3))
  (bind _returnvalue_3 (* _max_flight_range -1.0))
  (bind _returnvalue_4 (Math|Random|RandomFloatinRange _returnvalue_3 _max_flight_range))
  (Variables|Default|SetDelta%20Seconds DeltaSeconds)
  (if (Variables|Default|GetFlying%20Forward?)
    (Transformation|AddLocalOffset (Variables|Character|GetMesh) (* (Math|Vector|MakeVector (Variables|Default|GetForward%20Speed) 0.0 0.0) (Variables|Default|GetDelta%20Seconds)) false false)
    (Transformation|SetWorldRotation (Variables|Character|GetMesh) (Math|Interpolation|RInterpTo (Transformation|GetWorldRotation _mesh_2) (Math|Rotator|FindLookatRotation (Transformation|GetWorldLocation _mesh_2) (Transformation|GetWorldLocation (Variables|Default|GetFlight%20Target))) (Variables|Default|GetDelta%20Seconds) 1.2) false false)
    (if (Variables|Default|GetCollision%20On?)
      (Utilities|FlowControl|Delay 0.4)
      (bind (_outhit _returnvalue_5) (Class|KismetSystemLibrary|BoxTraceSingleforObjects (+ _returnvalue "0.000000,0.000000,60.000000") (- (+ _returnvalue (* (Math|Vector|GetForwardVector _mesh) 3e+02)) "0.000000,0.000000,-60.000000") "0.000000,80.000000,50.000000" (Transformation|GetWorldRotation (Variables|Character|GetMesh)) (Utilities|Array|MakeArray "ObjectTypeQuery2") true 0 "None" true "(R=1.000000,G=0.000000,B=0.000000,A=1.000000)" "(R=0.000000,G=1.000000,B=0.000000,A=1.000000)" 1.0))
      (if _returnvalue_5
        (bind _array_element (Utilities|Array|ForEachLoopwithBreak (Variables|Default|GetFruit%20REF%20Array) :!label _label)
          (:LoopBody
            (if (== _array_element (.HitActor (Collision|BreakHitResult _outhit)))
              (Utilities|FlowControl|Sequence
                (:then_0
                  (goto _label Break))
                (:then_1
                  (Variables|Default|SetFruit%20REF _array_element)))))
          (:Completed
            (Utilities|IsValid (Variables|Default|GetFruit%20REF)
              (:Is%20Valid
                (if (< (Math|Vector|VectorLength (- (.Location (Collision|BreakHitResult _outhit)) (Transformation|GetWorldLocation (Variables|Character|GetMesh)))) 1e+02)
                  (Variables|Default|SetCollision%20On? false)
                  (Variables|Default|SetFlying%20Forward? false)
                  (Utilities|IsValid (Variables|Default|GetFruit%20REF)
                    (:Is%20Valid
                      (Variables|Default|SetisEating true)
                      (Utilities|FlowControl|Sequence
                        (:then_0
                          (Components|MoveComponentTo (Variables|Character|GetMesh) "0.000000,0.000000,-49.000000" "0, 0, 0" true true 1.0 false))
                        (:then_1
                          (Components|MoveComponentTo (Variables|Collision|GetCapsuleComponent) (Transformation|GetWorldLocation (Variables|/Game/Fruit/Fruit.Fruit_C|GetBat%20platform (Variables|Default|GetFruit%20REF))) (Transformation|GetWorldRotation (Variables|/Game/Fruit/Fruit.Fruit_C|GetBat%20platform (Variables|Default|GetFruit%20REF))) true true 1.0 false)
                          (Utilities|FlowControl|Sequence
                            (:then_0
                              (Utilities|FlowControl|Delay (- (Variables|Default|GetTimeBatSpendsEatingInSeconds) 1.6))
                              (Variables|Default|SetisEating false)
                              (Utilities|FlowControl|Delay 1.0)
                              (Components|MoveComponentTo (Variables|Character|GetMesh) (Variables|Default|GetInitialMeshLocation) "0, 0, 0" true true 1.0 false))
                            (:then_1
                              (Components|MoveComponentTo (Variables|Collision|GetCapsuleComponent) (Transformation|GetWorldLocation (Variables|/Game/Fruit/Fruit.Fruit_C|GetBat%20platform (Variables|Default|GetFruit%20REF))) (Transformation|GetWorldRotation (Variables|/Game/Fruit/Fruit.Fruit_C|GetBat%20platform (Variables|Default|GetFruit%20REF))) true true (Variables|Default|GetTimeBatSpendsEatingInSeconds) false)
                              (Variables|Default|SetFruit%20REF 0)
                              (Variables|Default|SetCollision%20On? true)
                              (Variables|Default|SetFlying%20Forward? true)
                              (Variables|Default|SetTime%20in%20Flight 0)
                              (Variables|Default|SetAttractor%20Location "0, 0, 0")
                              (if (Variables|Default|GetFlying%20Forward?) :!label _label_2
                                (Transformation|SetRelativeLocation (Variables|Default|GetFlight%20Target) (Math|Vector|MakeVector (+ (.X (Math|Vector|BreakVector (Variables|Default|GetAttractor%20Location))) _returnvalue_4) (+ (.Y (Math|Vector|BreakVector (Variables|Default|GetAttractor%20Location))) _returnvalue_4) (+ (.Z (Math|Vector|BreakVector (Variables|Default|GetAttractor%20Location))) (Math|Random|RandomFloatinRange (* _max_flight_range -0.2) _max_flight_range))) false false)
                                (Variables|Default|SetTime%20in%20Flight (+ (Variables|Default|GetTime%20in%20Flight) 1))
                                (Math|Integer|CompareInt (Variables|Default|GetTime%20in%20Flight) 12
                                  (:>
                                    _)
                                  (:==
                                    _)
                                  (:<
                                    (Utilities|FlowControl|Delay (Math|Random|RandomFloatinRange 2.0 4.0))
                                    (goto _label_2)))
                                (Transformation|SetRelativeLocation (Variables|Default|GetFlight%20Target) (Variables|Default|GetAttractor%20Location) false false)))))))))))))
        (else
          (bind _returnvalue_6 (Class|KismetSystemLibrary|BoxTraceSingleforObjects (+ _returnvalue_2 "0.000000,0.000000,60.000000") (- (+ _returnvalue_2 (* (Math|Vector|GetForwardVector _mesh_3) 2e+02)) "0.000000,0.000000,-60.000000") "0.000000,20.000000,25.000000" (Transformation|GetWorldRotation (Variables|Character|GetMesh)) (Utilities|Array|MakeArray "ObjectTypeQuery1") true 0 "None" true "(R=0.161151,G=0.650845,B=1.000000,A=1.000000)" "(R=1.000000,G=0.819077,B=0.000000,A=1.000000)" 1.0))
          (if _returnvalue_6
            (Utilities|Time|SetTimerbyEvent (delegate Custom|Turn%20Back) 3.0)
            (Transformation|SetWorldLocation (Variables|Default|GetFlight%20Target) (Transformation|GetWorldLocation (Variables|Default|GetTurn%20Back%20Point)) false false)))))))

(event EventBeginPlay
  (Variables|Default|SetInitialMeshLocation (.location (Transformation|GetRelativeTransform (Variables|Character|GetMesh))))
  (bind _outactors (Actor|GetAllActorsOfClass "/Game/Fruit/Fruit.Fruit_C"))
  (Variables|Default|SetFruit%20REF%20Array _outactors))

(fn ConstructionScript
  (Transformation|SetRelativeLocation (Variables|Default|GetFlight%20Target) (Variables|Default|GetAttractor%20Location) false false))
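; BP_StaminaBoost is a pickup that gives stamina to BP_BatChar when the character overlaps it.
; Overlapping Sphere1 calls AddStamina with StaminaGain, disables that collision and hides the Sphere component.
; A fixed delay of a few seconds then restores visibility and collision, so the same actor is reused.
; Actor overlap also sets a Respawn flag, which these graphs never read.
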(event OnComponentBeginOverlap(Sphere1)
  (params (OverlappedComponent :type Primitive%20Component%20Object%20Reference) (OtherActor :type Actor%20Object%20Reference) (OtherComp :type Primitive%20Component%20Object%20Reference) (OtherBodyIndex :type Integer) (bFromSweep :type Boolean) (SweepResult :type Hit%20Result%20Structure%20%28by%20ref%29))
  (bind _asbp_bat_char (Utilities|Casting|CastToBP_BatChar OtherActor))
  (Utilities|IsValid _asbp_bat_char
    (:Is%20Valid
      (Default|AddStamina _asbp_bat_char (Variables|Default|GetStamina%20Gain))
      (Collision|SetCollisionEnabled (Variables|Default|GetSphere1) "NoCollision")
      (Rendering|SetVisibility (Variables|Default|GetSphere) false false)
      (Utilities|FlowControl|Delay 4.0)
      (Rendering|SetVisibility (Variables|Default|GetSphere) true false)
      (Collision|SetCollisionEnabled (Variables|Default|GetSphere1) "QueryAndPhysics"))))

(event EventBeginPlay)

(event Collision|EventActorBeginOverlap
  (params (OtherActor :type Actor%20Object%20Reference))
  (Variables|Default|SetRespawn true))

(event EventTick
  (params (DeltaSeconds :type Float%20%28single-precision%29)))

(fn ConstructionScript)
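; BP_Cauldron is a cauldron that consumes required ingredient items placed inside it until its ingredient set is empty.
; A Delay on Tick throttles overlap checks on InsideCollision for released BP_BaseItem actors with a needed IngredientType.
; A match is removed from IngredientList, printed, flagged as grabbed to block recounting, and destroyed after a delay.
; An empty set triggers a one-time completion debug message.
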(event EventBeginPlay)

(event EventTick
  (params (DeltaSeconds :type Float%20%28single-precision%29))
  (bind _ingredientlist (Variables|Default|GetIngredientList))
  (Utilities|FlowControl|Delay (Variables|Default|GetCollisionCheckRefreshTimer))
  (Utilities|FlowControl|Sequence
    (:then_0
      (for _array_element (Collision|GetOverlappingActors (Variables|Default|GetInside_Collision) "/Game/PigeonFlying/Blueprints/BP_BaseItem.BP_BaseItem_C" :!class /Script/Engine.PrimitiveComponent)
        (bind _asbp_base_item (Utilities|Casting|CastToBP_BaseItem _array_element))
        (Utilities|IsValid _asbp_base_item
          (:Is%20Valid
            (if (and (not (Variables|/Game/PigeonFlying/Blueprints/BP_BaseItem.BP_BaseItem_C|GetisGrabbed _asbp_base_item)) (Utilities|Set|Contains _ingredientlist (Variables|/Game/PigeonFlying/Blueprints/BP_BaseItem.BP_BaseItem_C|GetIngredientType _asbp_base_item)))
              (Utilities|Set|Remove _ingredientlist (Variables|/Game/PigeonFlying/Blueprints/BP_BaseItem.BP_BaseItem_C|GetIngredientType _asbp_base_item))
              (Development|PrintString (Utilities|String|EnumtoString (Variables|/Game/PigeonFlying/Blueprints/BP_BaseItem.BP_BaseItem_C|GetIngredientType _asbp_base_item)))
              (Variables|/Game/PigeonFlying/Blueprints/BP_BaseItem.BP_BaseItem_C|SetisGrabbed _asbp_base_item true)
              (Utilities|FlowControl|Delay (Variables|Default|GetItemDespawnTime))
              (Actor|DestroyActor _asbp_base_item))))))
    (:then_1
      (if (Utilities|Set|IsEmpty _ingredientlist)
        (Utilities|FlowControl|DoOnce false
          (:Completed
            (Development|PrintString "Cauldron thingy complete!" true true "(R=0.177594,G=1.000000,B=0.000000,A=1.000000)")))))))

(fn ConstructionScript)